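; BP_SkyController drives a comet-induced tint of the world's sky lighting.
; Each Tick it samples a curve at CometInfluence, caches the clamped CometRedAmount and pushes it to the MPC_Sky parameter collection.
; That amount lerps SkyAtmosphere ground albedo and SkyLight color between base and comet colors, recapturing the skylight every frame.
; BeginPlay finds the SkyAtmosphere and applies the initial parameter and albedo, while CometInfluence is only read here.
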(event EventBeginPlay
  ;[0.521 0.2159 0.05127] Kickoff/Execution
  (bind _returnvalue (Actor|GetActorOfClass "/Script/Engine.SkyAtmosphere"))
  (Variables|Default|SetSkyAtmosphereRef _returnvalue)
  ;[0.2159 0.117 0.3515] Cache Result (Comet Red Amount)
  (Variables|Default|SetCometRedAmount (Math|Curves|GetFloatValue (Variables|Default|GetCurve_CometRedSpike) (Variables|Default|GetCometInfluence)))
  ;[0.2159 0.117 0.3515] Push Parameter to MPC
  (Rendering|Material|SetScalarParameterValue "/Game/NexusSkies/03_World/Sky/Materials/MPC_Sky.MPC_Sky" "CometRedAmount" (Variables|Default|GetCometRedAmount) :!class /Script/Engine.KismetMaterialLibrary)
  ;[0.1878 0.1878 0.1878] Currently static - will be driven by CometRedAmount later
  (CallFunction|ApplyCometGroundAlbedo))

(event Collision|EventActorBeginOverlap
  (params (OtherActor :type Actor%20Object%20Reference)))

(event EventTick
  (params (DeltaSeconds :type Float%20%28single-precision%29))
  ;[0.521 0.2159 0.05127] Update Loop (Comet Sky)
  (CallFunction|UpdateCometSky))

(fn ConstructionScript)

(fn ApplyCometGroundAlbedo
  (bind _skyatmosphereref (Variables|Default|GetSkyAtmosphereRef))
  ;[0.5395 0.3564 0.06848] Validate SkyAtmosphereRef
  (Utilities|IsValid _skyatmosphereref
    (:Is%20Valid
      ;[0.15 0.05127 0.3515] Apply to SkyAtmosphere
      (Class|SkyAtmosphereComponent|SetGroundAlbedo (Variables|/Script/Engine.SkyAtmosphere|GetSkyAtmosphereComponent _skyatmosphereref) (Math|Conversions|ToColor(LinearColor) (Math|Color|Lerp(LinearColor) (Variables|Default|GetBaseGroundAlbedo) (Variables|Default|GetCometGroundAlbedo) (Math|Float|Clamp(Float) (Variables|Default|GetCometRedAmount))))))))

(fn UpdateCometSky
  (bind _curve_cometredspike (Variables|Default|GetCurve_CometRedSpike))
  (bind _cometinfluence (Variables|Default|GetCometInfluence))
  (bind _returnvalue (Math|Curves|GetFloatValue _curve_cometredspike _cometinfluence))
  (bind _returnvalue_2 (Math|Float|Clamp(Float) _returnvalue))
  ;[0.2159 0.117 0.3515] Cache + Push to MPC
  (Variables|Default|SetCometRedAmount _returnvalue_2)
  (Rendering|Material|SetScalarParameterValue "/Game/NexusSkies/03_World/Sky/Materials/MPC_Sky.MPC_Sky" "CometRedAmount" _returnvalue_2 :!class /Script/Engine.KismetMaterialLibrary)
  ;[0.2623 0.1559 0.1022] Apply to World (Ground + Skylight)
  (CallFunction|ApplyCometGroundAlbedo)
  (CallFunction|ApplyCometSkyLightTint))

(fn ApplyCometSkyLightTint
  (bind _skylightref (Variables|Default|GetSkyLightRef))
  (bind _returnvalue (Actor|GetComponentbyClass _skylightref "/Script/Engine.SkyLightComponent"))
  ;[0.5395 0.3564 0.06848] Validate References
  (Utilities|IsValid (Variables|Default|GetSkyLightRef)
    (:Is%20Valid
      (Utilities|IsValid _returnvalue
        (:Is%20Valid
          ;[0.107 0.04231 0.2623] Apply + Recapture
          (Rendering|Components|Light|SetLightColor _returnvalue (Math|Color|Lerp(LinearColor) (Variables|Default|GetBaseSkyTint) (Variables|Default|GetCometSkyTint) (Math|Float|Clamp(Float) (Variables|Default|GetCometRedAmount))))
          (Class|SkyLightComponent|RecaptureSky _returnvalue))
        (:Is%20Not%20Valid
          _)))
    (:Is%20Not%20Valid
      _))
  (return))