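; World cycle manager that keeps the game's world clock, tracking elapsed time, day number and time of day.
; Each Tick passes delta seconds to UpdateWorldTime, which scales them by TimeScale and accumulates absolute world seconds.
; From that total it derives a one-based day index using SecondsPerDay, plus the time of day in seconds and hours.
; It only updates these variables and drives no lighting or other actors itself.
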(event EventBeginPlay)

(event Collision|EventActorBeginOverlap
  (params (OtherActor :type Actor%20Object%20Reference)))

(event EventTick
  (params (DeltaSeconds :type Float%20%28single-precision%29))
  (CallFunction|UpdateWorldTime DeltaSeconds))

(fn ConstructionScript)

(fn UpdateWorldTime
  (params (A :type Float%20%28double-precision%29))
  (bind _secondsperday (Variables|Default|GetSecondsPerDay))
  ;[0.521 0.2159 0.05127] Function Entry / Inputs
  ;[0.09759 0.2542 0.09759] Time Delta Scaling
  (bind _output_get (Variables|Default|SetDeltaWorldTimeSeconds (* A (Variables|Default|GetTimeScale))))
  ;[0.2159 0.117 0.3515] Accumulate Absolute World Time
  (bind _output_get_2 (Variables|Default|SetWorldTimeSeconds (+ (Variables|Default|GetWorldTimeSeconds) _output_get)))
  (Utilities|FlowControl|Sequence
    (:then_0
      ;[0.09759 0.2542 0.09759] Compute Day Index
      (Variables|Default|SetDayIndex (+ (Math|Float|Floor (/ _output_get_2 _secondsperday)) 1)))
    (:then_1
      ;[0.09759 0.2542 0.09759] Compute Time Of Day Seconds
      (bind _output_get_3 (Variables|Default|SetTimeOfDaySeconds (Math|Float|%(Float) _output_get_2 _secondsperday)))
      ;[0.09759 0.2542 0.09759] Compute Time Of Day Hours
      (Variables|Default|SetTimeOfDayHours (/ _output_get_3 3.6e+03)))))