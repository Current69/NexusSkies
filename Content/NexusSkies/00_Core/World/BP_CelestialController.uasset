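; Celestial controller that rotates the referenced sunlight actor every tick from the world cycle manager's day index and hour.
; A cosine season curve sets day length, centering sunrise and sunset on noon in an FTimeState.
; Normalized day or night progress maps to sun pitch, with debug values printed each update.
; BuildTimeState's PeakDay and YearLength inputs are unused; the season math hardcodes its own.
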(event EventBeginPlay)

(event Collision|EventActorBeginOverlap
  (params (OtherActor :type Actor%20Object%20Reference)))

(event EventTick
  (params (DeltaSeconds :type Float%20%28single-precision%29))
  (CallFunction|UpdateSun))

(fn ConstructionScript)

(fn UpdateSun
  (bind _returnvalue (Math|Float|MakeLiteralFloat 9.0))
  (bind _returnvalue_2 (Math|Float|MakeLiteralFloat 15.5))
  (bind _worldcyclemanagerref (Variables|Default|GetWorldCycleManagerRef))
  (bind _dayindex (Variables|/Game/NexusSkies/00_Core/World/BP_WorldCycleManager.BP_WorldCycleManager_C|GetDayIndex _worldcyclemanagerref))
  (bind _timeofdayhours (Variables|/Game/NexusSkies/00_Core/World/BP_WorldCycleManager.BP_WorldCycleManager_C|GetTimeOfDayHours _worldcyclemanagerref))
  ;[0.521 0.2159 0.05127] Update Sun - Execution Entry
  ;[0.2159 0.117 0.3515] Cache Day / Hour (Local)
  (bind _output_get (LocalVariables|SetDay _dayindex))
  (LocalVariables|SetHour _timeofdayhours)
  (Development|PrintText (Utilities|Text|FormatText "Day {Day}   SeasonAlpha {Alpha}   DayLength {Length}" (Math|Conversions|ToFloat(Integer) _output_get) (.SeasonAlpha (CallFunction|ComputeDayLengthfromSeason (Math|Conversions|ToFloat(Integer) _output_get) _returnvalue _returnvalue_2)) (.DayLength (CallFunction|ComputeDayLengthfromSeason (Math|Conversions|ToFloat(Integer) _output_get) _returnvalue _returnvalue_2))))
  ;[0.2159 0.117 0.3515] Today's Day/Night Length
  (bind _output_get_2 (LocalVariables|SetDayLength (.DayLength (CallFunction|ComputeDayLengthfromSeason (Math|Conversions|ToFloat(Integer) _output_get) _returnvalue _returnvalue_2))))
  (LocalVariables|SetNightLength (- 24.0 _output_get_2))
  (bind _output_get_3 (Variables|Default|SetTimeState (CallFunction|BuildTimeState (Math|Conversions|ToFloat(Integer) _dayindex) _timeofdayhours _returnvalue _returnvalue_2 (Math|Float|MakeLiteralFloat 92.0) (Math|Float|MakeLiteralFloat 365.0))))
  (bind (_dayt _nightt _isday _pitchday _pitchnight) (CallFunction|ComputeDayNightProgression _output_get_3))
  (Development|PrintText (Utilities|Text|FormatText "Sunrise {Sunrise} Sunset {Sunset}" (.Sunrise (CallFunction|ComputeDayLengthfromSeason (Math|Conversions|ToFloat(Integer) _output_get) _returnvalue _returnvalue_2)) (.Sunset (CallFunction|ComputeDayLengthfromSeason (Math|Conversions|ToFloat(Integer) _output_get) _returnvalue _returnvalue_2))))
  (Development|PrintText (Utilities|Text|FormatText "Day T {DayT}   Night T {NightT}   Is Day {IsDay}   Pitch Day {PitchDay}   Pitch Night {PitchNight}" _dayt _nightt _isday _pitchday _pitchnight))
  ;[0.09759 0.2542 0.09759] Daytime Progression -> Sun Pitch Mapping
  (LocalVariables|SetDayT _dayt)
  (LocalVariables|SetPitchDay _pitchday)
  ;[0.09759 0.2542 0.09759] Night Pitch Mapping
  (LocalVariables|SetNightT _nightt)
  (LocalVariables|SetPitchNight _pitchnight)
  (LocalVariables|SetbIsDay _isday)
  ;[0.15 0.15 0.15 0.5] Apply Sun Rotation
  (CallFunction|ApplySunRotation (Math|Float|SelectFloat _pitchday _pitchnight _isday)))

(fn ComputeDayNightProgression
  (params (TimeState :type F%20Time%20State%20Structure))
  (bind (_hour _day _sunrise _sunset _daylength _nightlength) (Utilities|Struct|BreakFTimeState TimeState))
  (bind _returnvalue (- _hour _sunset))
  (bind _returnvalue_2 (- _hour _sunrise))
  (bind _returnvalue_3 (- 24.0 _sunset))
  (bind _returnvalue_4 (>= _hour _sunset))
  (bind _returnvalue_5 (/ _returnvalue_2 _daylength))
  (bind _returnvalue_6 (+ _hour _returnvalue_3))
  (bind _returnvalue_7 (Math|Float|SelectFloat _returnvalue _returnvalue_6 _returnvalue_4))
  (bind _returnvalue_8 (Math|Float|Clamp(Float) _returnvalue_5))
  (bind _returnvalue_9 (/ _returnvalue_7 _nightlength))
  (bind _returnvalue_10 (Math|Float|Clamp(Float) _returnvalue_9))
  (return _returnvalue_8 _returnvalue_10 (and (<= _hour _sunset) (>= _hour _sunrise)) (Math|Float|Lerp -9e+01 9e+01 _returnvalue_8) (Math|Float|Lerp 9e+01 2.7e+02 _returnvalue_10)))

(fn ComputeSeasonAlpha
  (params (Peak%20Day :type Float%20%28double-precision%29) (Year%20Length :type Float%20%28double-precision%29) (Day :type Float%20%28double-precision%29))
  (return (Math|Trig|Cos(Radians) (* (/ (- Day Peak%20Day) Year%20Length) (* 2.0 (Math|Trig|GetPI))))))

(fn ComputeDayMid
  (params (MinDay :type Float%20%28double-precision%29) (MaxDay :type Float%20%28double-precision%29))
  (return (/ (+ MinDay MaxDay) 2.0)))

(fn ComputeDayAmp
  (params (MinDay :type Float%20%28double-precision%29) (MaxDay :type Float%20%28double-precision%29))
  (return (/ (- MaxDay MinDay) 2.0)))

(fn ComputeDayLengthfromSeason
  (params (Day :type Float%20%28double-precision%29) (MinDay :type Float%20%28double-precision%29) (MaxDay :type Float%20%28double-precision%29))
  (bind _seasonalpha (CallFunction|ComputeSeasonAlpha 172.0 365.0 Day))
  (bind _mid (CallFunction|ComputeDayMid MinDay MaxDay))
  (bind _amp (CallFunction|ComputeDayAmp MinDay MaxDay))
  (bind _returnvalue (* _amp _seasonalpha))
  (bind _returnvalue_2 (+ _mid _returnvalue))
  (bind (_sunrise _sunset) (CallFunction|ComputeSunriseSunset _returnvalue_2))
  (return _returnvalue_2 (Math|Float|Clamp(Float) _seasonalpha) _sunrise _sunset))

(fn ComputeSunriseSunset
  (params (DayLength :type Float%20%28double-precision%29))
  (bind _returnvalue (Math|Float|Clamp(Float) DayLength 0.1 23.9))
  (bind _returnvalue_2 (/ _returnvalue 2.0))
  (return (- 12.0 _returnvalue_2) (+ 12.0 _returnvalue_2)))

(fn BuildTimeState
  (params (Day :type Float%20%28double-precision%29) (Hour :type Float%20%28double-precision%29) (MinDay :type Float%20%28double-precision%29) (MaxDay :type Float%20%28double-precision%29) (PeakDay :type Float%20%28double-precision%29) (YearLength :type Float%20%28double-precision%29))
  (bind (_daylength _seasonalpha _sunrise _sunset) (CallFunction|ComputeDayLengthfromSeason Day MinDay MaxDay))
  (return (Utilities|Struct|MakeFTimeState Hour (Math|Float|Truncate Day) _sunrise _sunset _daylength (- 24.0 _daylength) _seasonalpha)))

(fn ApplySunRotation
  (params (FinalPitch :type Float%20%28double-precision%29))
  (Transformation|SetActorRotation (Variables|Default|GetSunlightRef) (Math|Rotator|MakeRotator 0.0 (+ FinalPitch -9e+01) 9e+01)))